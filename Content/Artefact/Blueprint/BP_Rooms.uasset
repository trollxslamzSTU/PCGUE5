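; BP_Rooms is a room Blueprint that prepares seed and position data for procedural room generation.
; On construction it calls ResetSeed, then caches the actor's location in Position.
; Unless KeepExteriorWallShape is set, ResetSeed rolls a new Seed and derives the room generation point count from a stream seeded with it.
; The generation itself is not in this Blueprint's graphs, and its BeginPlay, overlap and Tick events are empty.
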(event `ResetSeed`
  (if (not (`self.KeepExteriorWallShape`))
    (set `self.Seed` (`KismetMathLibrary.RandomIntegerInRange` 0 2556789))
    (set `self.AmountOfPointsForRoomGeneration` (`KismetMathLibrary.RandomIntegerInRangeFromStream` (`KismetMathLibrary.MakeRandomStream` (`self.Seed`)) 8 16))))

(fn `GetPostion`
  (set `self.Position` (`self.K2_GetActorLocation`)))

(fn `UserConstructionScript`
  (`self.ResetSeed`)
  (`self.GetPostion`))