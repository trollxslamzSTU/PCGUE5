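; PCG Blueprint element that picks a random subset of input points, likely for wall placement going by its name.
; For each InPoints data, it shuffles the points with the context's seeded random stream and keeps either a controlled count or a clamped, rounded-up percentage.
; It outputs NewPoints and NonChosenPoints, but both receive the chosen points, and the chosen array is never cleared between inputs.
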(fn Execute
  (params (Input :type PCG%20Data%20Collection%20Structure%20%28by%20ref%29))
  (bind _array (Utilities|Array|MakeArray))
  (bind _collection (LocalVariables|GetCollection))
  (bind _returnvalue (Data|GetTypedInputsbyPinLabel Input "InPoints" "/Script/PCG.PCGPointData"))
  (for _array_element _returnvalue
    (bind _output_get (LocalVariables|SetInData _array_element))
    (bind _output_get_2 (LocalVariables|SetInPoints (SpatialData|GetPoints _output_get)))
    (LocalVariables|SetNumPointsWhichAreKept (Math|Integer|Min(Integer) (Utilities|Array|Length _output_get_2) (select (Variables|Default|GetControlled) (Variables|Default|GetControlledAmount) (Math|Float|Ceil (* (Utilities|Array|Length _output_get_2) (Math|Float|Clamp(Float) (Variables|Default|GetPercentAmount)))))))
    (bind _returnvalue_2 (Class|PCGBlueprintElement|GetRandomStream (SoundLibrary|GetContext)))
    (Utilities|Array|ShuffleFromStream (LocalVariables|GetInPoints) _returnvalue_2)
    (for (_array_element_2 _array_index) (LocalVariables|GetInPoints)
      (Utilities|Array|Add (select (>= _array_index (LocalVariables|GetNumPointsWhichAreKept)) (LocalVariables|GetNonChosenPoints) (LocalVariables|GetChosenPoints)) _array_element_2))
    (bind _returnvalue_3 (Game|ConstructObjectfromClass "/Script/PCG.PCGPointData"))
    (bind _output_get_3 (LocalVariables|SetChosenPointData _returnvalue_3))
    (SpatialData|InitializefromData _output_get_3 (LocalVariables|GetInData) 0 true true)
    (SpatialData|SetPoints (LocalVariables|GetChosenPointData) (LocalVariables|GetChosenPoints))
    (bind _returnvalue_4 (Game|ConstructObjectfromClass "/Script/PCG.PCGPointData"))
    (bind _output_get_4 (LocalVariables|SetNonChosenPointData _returnvalue_4))
    (SpatialData|InitializefromData _output_get_4 (LocalVariables|GetInData) 0 true true)
    (SpatialData|SetPoints (LocalVariables|GetNonChosenPointData) (LocalVariables|GetChosenPoints))
    (Class|PCGDataFunctionLibrary|AddtoCollection _collection (LocalVariables|GetChosenPointData) "NewPoints" _array)
    (Class|PCGDataFunctionLibrary|AddtoCollection _collection (LocalVariables|GetNonChosenPointData) "NonChosenPoints" _array))
  (return (LocalVariables|GetCollection)))