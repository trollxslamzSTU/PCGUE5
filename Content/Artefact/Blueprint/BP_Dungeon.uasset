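; Dungeon layout actor that builds a path on a spline from forward, left and right steps and runs PCG generation on it.
; Each step appends a linear point and records its direction, blocking direct left-right reversals.
; GenerateCorridors, despite its name, line-traces each segment and again past the hit in the recorded direction, spawning tagged door actors at hits.
; Corridor spawning and AddCorridor calls are disconnected.
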(event Custom|GenerateForward
  (Variables|Default|SetLastInput "Forward")
  (CallFunction|AddSplinePopint (Variables|Default|GetForward) 0.0))

(event Custom|GenerateRight
  (if (not (Utilities|Enum|Equal(Enum) (Variables|Default|GetLastInput) "Left"))
    (Variables|Default|SetLastInput "Right")
    (CallFunction|AddSplinePopint 0.0 (Variables|Default|GetRight))))

(event Custom|GenerateDungeon
  (PCG|Generate (Variables|Default|GetPCG) true))

(event Custom|GenerateLeft
  (if (not (Utilities|Enum|Equal(Enum) (Variables|Default|GetLastInput) "Right"))
    (Variables|Default|SetLastInput "Left")
    (CallFunction|AddSplinePopint 0.0 (Variables|Default|GetLeft))))

(event Custom|GenerateCorridors
  (for _index (range 0 (Spline|GetNumberOfSplinePoints (Variables|Default|GetSpline)))
    (bind (_outhit _returnvalue) (Collision|LineTraceByChannel (+ (+ (Transformation|GetWorldLocation (Variables|Default|GetSpline)) (.position (Spline|GetSplinePointAt (Variables|Default|GetSpline) _index "Local"))) (Math|Vector|MakeVector 0.0 0.0 3e+02)) (+ (+ (.position (Spline|GetSplinePointAt (Variables|Default|GetSpline) (+ _index 1) "Local")) (Transformation|GetWorldLocation (Variables|Default|GetSpline))) (Math|Vector|MakeVector 0.0 0.0 3e+02)) "TraceTypeQuery3" true 0 "None"))
    (if _returnvalue
      (bind _returnvalue_2 (Game|SpawnActorfromClass "/Game/Artefact/Blueprint/BP_DoorDiff.BP_DoorDiff_C" (Math|Transform|MakeTransform (- (.Location (Collision|BreakHitResult _outhit)) (Math|Vector|MakeVector 0.0 0.0 2.5e+02)) "0, 0, 0" "1.000000,1.000000,1.000000") "Undefined" "MultiplyWithRoot" 0 0))
      (Utilities|Array|Add (Variables|/Script/Engine.Actor|GetTags _returnvalue_2) "")
      (Utilities|Array|SetArrayElem (Variables|/Script/Engine.Actor|GetTags _returnvalue_2) 0 "SpawnedbyPCG")
      (Development|PrintString (Utilities|String|ToString(Boolean) (.ReturnValue (Utilities|Map|Find (Variables|Default|GetInputMap) _index))))
      (switch string (.Value (Utilities|Map|Find (Variables|Default|GetInputMap) _index))
        (:Forward
          (bind (_outhit_2 _returnvalue_3) (Collision|LineTraceByChannel (+ (.Location (Collision|BreakHitResult _outhit)) "200.000000,0.000000,0.000000") (+ (+ (+ (.position (Spline|GetSplinePointAt (Variables|Default|GetSpline) (+ _index 1) "Local")) (Transformation|GetWorldLocation (Variables|Default|GetSpline))) (Math|Vector|MakeVector 0.0 0.0 3e+02)) "1000.000000,0.000000,0.000000") "TraceTypeQuery3" false 0 "ForDuration"))
          (if _returnvalue_3
            (bind _returnvalue_4 (Game|SpawnActorfromClass "/Game/Artefact/Blueprint/BP_DoorDiff.BP_DoorDiff_C" (Math|Transform|MakeTransform (- (.Location (Collision|BreakHitResult _outhit_2)) (Math|Vector|MakeVector 0.0 0.0 2.5e+02)) "0, 0, 0" "1.000000,1.000000,1.000000") "Undefined" "MultiplyWithRoot" 0 0))
            (Utilities|Array|Add (Variables|/Script/Engine.Actor|GetTags _returnvalue_4) "")
            (Utilities|Array|SetArrayElem (Variables|/Script/Engine.Actor|GetTags _returnvalue_4) 0 "SpawnedbyPCG")))
        (:Left
          (bind (_outhit_3 _returnvalue_5) (Collision|LineTraceByChannel (+ (.Location (Collision|BreakHitResult _outhit)) "0.000000,-200.000000,0.000000") (+ (+ (+ (.position (Spline|GetSplinePointAt (Variables|Default|GetSpline) (+ _index 1) "Local")) (Transformation|GetWorldLocation (Variables|Default|GetSpline))) (Math|Vector|MakeVector 0.0 0.0 3e+02)) "0.000000,-1000.000000,0.000000") "TraceTypeQuery3" false 0 "ForDuration"))
          (if _returnvalue_5
            (bind _returnvalue_6 (Game|SpawnActorfromClass "/Game/Artefact/Blueprint/BP_DoorDiff.BP_DoorDiff_C" (Math|Transform|MakeTransform (- (.Location (Collision|BreakHitResult _outhit_3)) (Math|Vector|MakeVector 0.0 0.0 2.5e+02)) "0, 0, 0" "1.000000,1.000000,1.000000") "Undefined" "MultiplyWithRoot" 0 0))
            (Utilities|Array|Add (Variables|/Script/Engine.Actor|GetTags _returnvalue_6) "")
            (Utilities|Array|SetArrayElem (Variables|/Script/Engine.Actor|GetTags _returnvalue_6) 0 "SpawnedbyPCG")))
        (:Right
          (bind (_outhit_4 _returnvalue_7) (Collision|LineTraceByChannel (+ (.Location (Collision|BreakHitResult _outhit)) "0.000000,200.000000,0.000000") (+ (+ (+ (.position (Spline|GetSplinePointAt (Variables|Default|GetSpline) (+ _index 1) "Local")) (Transformation|GetWorldLocation (Variables|Default|GetSpline))) (Math|Vector|MakeVector 0.0 0.0 3e+02)) "0.000000,1000.000000,0.000000") "TraceTypeQuery3" false 0 "ForDuration"))
          (if _returnvalue_7
            (bind _returnvalue_8 (Game|SpawnActorfromClass "/Game/Artefact/Blueprint/BP_DoorDiff.BP_DoorDiff_C" (Math|Transform|MakeTransform (- (.Location (Collision|BreakHitResult _outhit_4)) (Math|Vector|MakeVector 0.0 0.0 2.5e+02)) "0, 0, 0" "1.000000,1.000000,1.000000") "Undefined" "MultiplyWithRoot" 0 0))
            (Utilities|Array|Add (Variables|/Script/Engine.Actor|GetTags _returnvalue_8) "")
            (Utilities|Array|SetArrayElem (Variables|/Script/Engine.Actor|GetTags _returnvalue_8) 0 "SpawnedbyPCG")))))))

(fn ConstructionScript)

(fn AddSplinePopint
  (params (XPos :type Float%20%28double-precision%29) (YPos :type Float%20%28double-precision%29))
  (bind _spline (Variables|Default|GetSpline))
  (bind _spline_2 (Variables|Default|GetSpline))
  (bind _returnvalue (Spline|GetNumberOfSplinePoints _spline))
  (bind _returnvalue_2 (- _returnvalue 1))
  (Utilities|Map|Add (Variables|Default|GetInputMap) _returnvalue_2 (Variables|Default|GetLastInput))
  (Spline|AddSplinePoint _spline_2 (+ (.position (Spline|GetSplinePointAt _spline _returnvalue_2 "Local")) (Math|Vector|MakeVector XPos YPos 0.0)) "Local" true)
  (Spline|SetSplinePointType _spline_2 (- (Spline|GetNumberOfSplinePoints (Variables|Default|GetSpline)) 1) "Linear" true))

(fn AddCorridor
  (params (XPos :type Float%20%28double-precision%29) (YPos :type Float%20%28double-precision%29))
  (bind _spline (Variables|Default|GetSpline))
  (bind _spline_2 (Variables|Default|GetSpline))
  (bind _returnvalue (Transformation|GetWorldLocation _spline))
  (bind _returnvalue_2 (Spline|GetNumberOfSplinePoints _spline_2))
  (bind _returnvalue_3 (- _returnvalue_2 1))
  (bind _returnvalue_4 (Spline|GetSplinePointAt _spline_2 _returnvalue_3 "Local"))
  (bind _returnvalue_5 (+ _returnvalue (.position _returnvalue_4)))
  (bind _returnvalue_6 (- _returnvalue_5 (Math|Vector|MakeVector XPos YPos 0.0)))
  (Collision|MultiLineTraceByChannel (+ _returnvalue_6 (Math|Vector|MakeVector 0.0 0.0 3e+02)) (+ _returnvalue_6 (Math|Vector|MakeVector XPos YPos 3e+02)) "TraceTypeQuery3" true 0 "ForDuration"))