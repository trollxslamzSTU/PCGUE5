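; BP_Corridor is a corridor actor that builds straight sections of floor and walls from mesh instances.
; Three custom events extend it forward, left or right, each adding one Floor, LeftWall and RightWall instance from a given location and index.
; Wall positions use hard-coded offsets plus an index-based step, with RightWall X and Y negated and side-direction walls yawed a quarter turn.
; BeginPlay, Tick and the construction script are empty.
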(event `AddInstanceForward`
  (params (Location :type "Vector Structure") (Index :type Integer))
  (bind _returnvalue (* Index 285))
  (bind _scale (`self.Scale`))
  (bind (_loc_x _loc_y _loc_z) (`KismetMathLibrary.BreakVector` (`self.Loc`)))
  (bind (_loc_x_2 _loc_y_2 _loc_z_2) (`KismetMathLibrary.BreakVector` (`self.Loc`)))
  (bind (_loc_x_3 _loc_y_3 _loc_z_3) (`KismetMathLibrary.BreakVector` (`self.Loc`)))
  (bind (_loc_x_4 _loc_y_4 _loc_z_4) (`KismetMathLibrary.BreakVector` (`self.Loc`)))
  (set `self.Loc` Location)
  (`InstancedStaticMeshComponent.AddInstance` (`self.Floor`) (`KismetMathLibrary.MakeTransform` (`self.Loc`)) false)
  (if (== Index 0)
    (`InstancedStaticMeshComponent.AddInstance` (`self.LeftWall`) (`KismetMathLibrary.MakeTransform` (`KismetMathLibrary.MakeVector` (+ _loc_x 15.0) _loc_y _loc_z) (struct) _scale) false)
    (`InstancedStaticMeshComponent.AddInstance` (`self.RightWall`) (`KismetMathLibrary.MakeTransform` (`KismetMathLibrary.MakeVector` (* (+ _loc_x_2 15.0) -1.0) (* _loc_y_2 -1.0) _loc_z_2) (struct) _scale) false)
    (else
      (`InstancedStaticMeshComponent.AddInstance` (`self.LeftWall`) (`KismetMathLibrary.MakeTransform` (`KismetMathLibrary.MakeVector` (+ (+ _loc_x_3 _returnvalue) 15.0) _loc_y_3 _loc_z_3) (struct) _scale) false)
      (`InstancedStaticMeshComponent.AddInstance` (`self.RightWall`) (`KismetMathLibrary.MakeTransform` (`KismetMathLibrary.MakeVector` (* (+ (+ _loc_x_4 _returnvalue) 15.0) -1.0) (* _loc_y_4 -1.0) _loc_z_4) (struct) _scale) false))))

(event `AddInstanceLeft`
  (params (Location :type "Vector Structure") (Index :type Integer))
  (bind _returnvalue (* Index 285))
  (bind _scale (`self.Scale`))
  (bind (_loc_x _loc_y _loc_z) (`KismetMathLibrary.BreakVector` (`self.Loc`)))
  (bind (_loc_x_2 _loc_y_2 _loc_z_2) (`KismetMathLibrary.BreakVector` (`self.Loc`)))
  (bind (_loc_x_3 _loc_y_3 _loc_z_3) (`KismetMathLibrary.BreakVector` (`self.Loc`)))
  (bind (_loc_x_4 _loc_y_4 _loc_z_4) (`KismetMathLibrary.BreakVector` (`self.Loc`)))
  (set `self.Loc` Location)
  (`InstancedStaticMeshComponent.AddInstance` (`self.Floor`) (`KismetMathLibrary.MakeTransform` (`self.Loc`)) false)
  (if (== Index 0)
    (`InstancedStaticMeshComponent.AddInstance` (`self.LeftWall`) (`KismetMathLibrary.MakeTransform` (`KismetMathLibrary.MakeVector` (+ _loc_x 250.0) (+ _loc_y 235.0) _loc_z) (struct :`Yaw` 90.0) _scale) false)
    (`InstancedStaticMeshComponent.AddInstance` (`self.RightWall`) (`KismetMathLibrary.MakeTransform` (`KismetMathLibrary.MakeVector` (* (- _loc_x_2 250.0) -1.0) (* (- _loc_y_2 255.0) -1.0) _loc_z_2) (struct :`Yaw` 90.0) _scale) false)
    (else
      (`InstancedStaticMeshComponent.AddInstance` (`self.LeftWall`) (`KismetMathLibrary.MakeTransform` (`KismetMathLibrary.MakeVector` (+ _loc_x_3 250.0) (+ (- _loc_y_3 _returnvalue) 240.0) _loc_z_3) (struct :`Yaw` 90.0) _scale) false)
      (`InstancedStaticMeshComponent.AddInstance` (`self.RightWall`) (`KismetMathLibrary.MakeTransform` (`KismetMathLibrary.MakeVector` (* (- _loc_x_4 250.0) -1.0) (* (- (- _loc_y_4 _returnvalue) 250.0) -1.0) _loc_z_4) (struct :`Yaw` 90.0) _scale) false))))

(event `AddInstanceRight`
  (params (Location :type "Vector Structure") (Index :type Integer))
  (bind _returnvalue (* Index 285))
  (bind _scale (`self.Scale`))
  (bind (_loc_x _loc_y _loc_z) (`KismetMathLibrary.BreakVector` (`self.Loc`)))
  (bind (_loc_x_2 _loc_y_2 _loc_z_2) (`KismetMathLibrary.BreakVector` (`self.Loc`)))
  (bind (_loc_x_3 _loc_y_3 _loc_z_3) (`KismetMathLibrary.BreakVector` (`self.Loc`)))
  (bind (_loc_x_4 _loc_y_4 _loc_z_4) (`KismetMathLibrary.BreakVector` (`self.Loc`)))
  (set `self.Loc` Location)
  (`InstancedStaticMeshComponent.AddInstance` (`self.Floor`) (`KismetMathLibrary.MakeTransform` (`self.Loc`)) false)
  (if (== Index 0)
    (`InstancedStaticMeshComponent.AddInstance` (`self.LeftWall`) (`KismetMathLibrary.MakeTransform` (`KismetMathLibrary.MakeVector` (+ _loc_x_3 250.0) (+ _loc_y_3 250.0) _loc_z_3) (struct :`Yaw` 90.0) _scale) false)
    (`InstancedStaticMeshComponent.AddInstance` (`self.RightWall`) (`KismetMathLibrary.MakeTransform` (`KismetMathLibrary.MakeVector` (* (- _loc_x_4 250.0) -1.0) (* (- _loc_y_4 235.0) -1.0) _loc_z_4) (struct :`Yaw` 90.0) _scale) false)
    (else
      (`InstancedStaticMeshComponent.AddInstance` (`self.LeftWall`) (`KismetMathLibrary.MakeTransform` (`KismetMathLibrary.MakeVector` (+ _loc_x 250.0) (+ (+ _loc_y _returnvalue) 245.0) _loc_z) (struct :`Yaw` 90.0) _scale) false)
      (`InstancedStaticMeshComponent.AddInstance` (`self.RightWall`) (`KismetMathLibrary.MakeTransform` (`KismetMathLibrary.MakeVector` (* (- _loc_x_2 250.0) -1.0) (* (- (+ _loc_y_2 _returnvalue) 235.0) -1.0) _loc_z_2) (struct :`Yaw` 90.0) _scale) false))))

(fn `UserConstructionScript`)